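; Standard game mode that sets up a crystal-retrieval escape level with a void hazard.
; On BeginPlay it caches GI_Standard, prints the controls and objective, and spawns a large, scaled BP_VoidFill below the origin.
; It also spawns and plays the Explore ambient sound, handing that actor to the game instance.
; Each tick it delegates void height updates and kill checks to the game instance.
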(event EventBeginPlay
  (bind _asgi_standard (Utilities|Casting|CastToGI_Standard (Game|GetGameInstance)))
  (Variables|Default|SetGameInstance _asgi_standard)
  (Development|PrintString "Press 'E' on a Keyboard or X on a controller to interact with objects" true true "(R=0.000000,G=0.660000,B=1.000000,A=1.000000)" 5.0)
  (Development|PrintString "Collect the Red Crystal and Return Here to Escape." true true "(R=0.000000,G=0.660000,B=1.000000,A=1.000000)" 5.0)
  (Game|SpawnActorfromClass "/Game/Objects/VoidPlane/BP_VoidFill.BP_VoidFill_C" (Math|Transform|MakeTransform (Math|Vector|MakeVector 0.0 1.0 -6.4e+02) "0, 0, 0" "150.000000,20.000000,20.000000") "Undefined" 0 0)
  (bind _returnvalue (Game|SpawnActorfromClass "/Script/Engine.AmbientSound" (Math|Transform|MakeTransform "0, 0, 0") "Undefined" 0 0))
  (Audio|Components|Audio|SetSound (Variables|/Script/Engine.AmbientSound|GetAudioComponent _returnvalue) "/Game/Music/Explore.Explore")
  (Audio|Components|Audio|Play (Variables|/Script/Engine.AmbientSound|GetAudioComponent _returnvalue) 0.0)
  (Variables|/Game/GameInstances/GI_Standard.GI_Standard_C|SetSound (Variables|Default|GetGameInstance) _returnvalue))

(event EventTick
  (params (DeltaSeconds :type Float%20%28single-precision%29))
  (bind _gameinstance (Variables|Default|GetGameInstance))
  (Default|UpdateVoidHeight _gameinstance DeltaSeconds)
  (Default|CheckVoidKill _gameinstance))

(fn ConstructionScript)