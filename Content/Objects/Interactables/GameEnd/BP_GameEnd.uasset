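; BP_GameEnd is an interactable trigger actor that ends the game in a win when the player reaches it.
; On BeginPlay it caches the GI_Standard game instance.
; On overlap it checks the game instance's CanWin flag and that the overlapping actor is the player pawn, then calls Win on the game instance with the BP_Player.
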(event EventBeginPlay
  (bind _asgi_standard (Utilities|Casting|CastToGI_Standard (Game|GetGameInstance)))
  (Variables|Default|SetGameInstance _asgi_standard))

(event Collision|EventActorBeginOverlap
  (params (OtherActor :type Actor%20Object%20Reference))
  (bind _returnvalue (Game|Player|GetPlayerPawn 0))
  (if (Variables|/Game/GameInstances/GI_Standard.GI_Standard_C|GetCanWin (Variables|Default|GetGameInstance))
    (if (== OtherActor _returnvalue)
      (bind _asbp_player (Utilities|Casting|CastToBP_Player _returnvalue))
      (Default|Win (Variables|Default|GetGameInstance) _asbp_player))))

(event EventTick
  (params (DeltaSeconds :type Float%20%28single-precision%29)))

(fn ConstructionScript)