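; BP_VoidPlane is the void plane that rises through the level to match the void height tracked by GI_Standard.
; Once StartClimb enables climbing, Tick reads that height from the cached game instance and snaps the sprite's Z to it plus a correction offset.
; It only moves the sprite upward, keeping X and Y, and stops updating while the game instance's End flag is set.
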(event EventBeginPlay
  (bind _asgi_standard (Utilities|Casting|CastToGI_Standard (Game|GetGameInstance)))
  (Variables|Default|SetGameInstance _asgi_standard))

(event EventStartClimb
  (Variables|Default|SetCanClimb true))

(event EventTick
  (params (DeltaSeconds :type Float%20%28single-precision%29))
  (bind _sprite (Variables|Default|GetSprite))
  (bind _gameinstance (Variables|Default|GetGameInstance))
  (bind _heightcorection (Variables|Default|GetHeightCorection))
  (bind _returnvalue (Transformation|GetWorldLocation _sprite))
  (bind (_x _y _z) (Math|Vector|BreakVector _returnvalue))
  (if (Variables|Default|GetCanClimb)
    (if (not (Variables|/Game/GameInstances/GI_Standard.GI_Standard_C|GetEnd _gameinstance))
      (bind _height (Default|GetVoidHeight _gameinstance))
      (if (< (- _z _heightcorection) _height)
        (Transformation|SetWorldLocation (Variables|Default|GetSprite) (Math|Vector|MakeVector _x _y (+ _height _heightcorection)) false false)))))

(fn ConstructionScript)