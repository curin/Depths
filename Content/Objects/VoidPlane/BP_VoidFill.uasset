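; BP_VoidFill is a Paper2D sprite object that rises with the void height held by the game instance.
; BeginPlay caches GI_Standard, and a StartClimb event enables the per-tick climb.
; While the game instance's End flag is unset, Tick snaps the sprite's Z to the void height plus HeightCorrection, only ever moving it upward and leaving X and Y unchanged.
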(event EventBeginPlay
  (bind _asgi_standard (Utilities|Casting|CastToGI_Standard (Game|GetGameInstance)))
  (Variables|Default|SetGame%20Instance _asgi_standard))

(event EventStartClimb
  (Variables|Default|SetCan%20Climb true))

(event EventTick
  (params (DeltaSeconds :type Float%20%28single-precision%29))
  (bind _height_correction (Variables|Default|GetHeight%20Correction))
  (bind _game_instance (Variables|Default|GetGame%20Instance))
  (bind _papersprite (Variables|Default|GetPaperSprite))
  (bind _returnvalue (Transformation|GetWorldLocation _papersprite))
  (bind (_x _y _z) (Math|Vector|BreakVector _returnvalue))
  (if (Variables|Default|GetCan%20Climb)
    (if (not (Variables|/Game/GameInstances/GI_Standard.GI_Standard_C|GetEnd _game_instance))
      (bind _height (Default|GetVoidHeight _game_instance))
      (if (< (- _z _height_correction) _height)
        (Transformation|SetWorldLocation (Variables|Default|GetPaperSprite) (Math|Vector|MakeVector _x _y (+ _height _height_correction)) false false)))))

(fn ConstructionScript)