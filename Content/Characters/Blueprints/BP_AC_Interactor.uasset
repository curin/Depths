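; An actor component that lets its owner detect and trigger nearby interactable objects.
; Every tick it runs a sphere trace at the owner's location against a single object type, storing whether something was hit and which actor.
; Its Interact event, when a target is available, sends that actor an InteractMessage with the owning Pawn.
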(event Custom|Interact
  (if (Variables|Default|GetCanInteract)
    (bind _aspawn (Utilities|Casting|CastToPawn (Components|GetOwner)))
    (Class|IInteractable|Interact(Message) (Variables|Default|GetInteractable) _aspawn)))

(event EventBeginPlay)

(event EventTick
  (params (DeltaSeconds :type Float%20%28single-precision%29))
  (CallFunction|CheckInteractDistance))

(fn CheckInteractDistance
  (bind _returnvalue (Components|GetOwner))
  (bind _returnvalue_2 (Transformation|GetActorLocation _returnvalue))
  (bind (_outhit _returnvalue_3) (Collision|SphereTraceForObjects _returnvalue_2 _returnvalue_2 (Variables|Default|GetInteractDistance) (Utilities|Array|MakeArray "ObjectTypeQuery9") false 0 (Variables|Default|GetDebugDraw)))
  (Variables|Default|SetCanInteract _returnvalue_3)
  (Variables|Default|SetInteractable (.HitActor (Collision|BreakHitResult _outhit))))