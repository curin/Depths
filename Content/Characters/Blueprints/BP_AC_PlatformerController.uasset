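; Platformer character controller component that drives horizontal movement, jumping and ground detection through a Mover object.
; On BeginPlay it sets up horizontal motion and either a simple or exponential jump model, chosen by the Simple flag.
; Each tick it feeds X input with a dead zone to the Mover and runs a head check.
; It then updates the active jump or, when not jumping, runs a coyote-time ground check.
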(event EventBeginPlay
  (bind _mover (Variables|Default|GetMover))
  (bind _terminalvelocitymult (Variables|Default|GetTerminalVelocityMult))
  (bind _jumpcontrolpercent (Variables|Default|GetJumpControlPercent))
  (Default|XConstruct _mover)
  (if (Variables|Default|GetSimple)
    (Default|SimpleConstruct _mover _terminalvelocitymult _jumpcontrolpercent)
    (else
      (Default|ExponentialConstruct _mover _terminalvelocitymult _jumpcontrolpercent))))

(event EventTick
  (params (DeltaSeconds :type Float%20%28single-precision%29))
  (bind _mover (Variables|Default|GetMover))
  (Default|XMotion _mover DeltaSeconds (Variables|Default|GetX%20Input) (Variables|Default|GetDeadZone))
  (Default|HeadCheck _mover)
  (if (Variables|/Game/Characters/Blueprints/BP_AC_Mover.BP_AC_Mover_C|GetIsJumping _mover)
    (if (Variables|Default|GetSimple)
      (Default|SimpleJump _mover)
      (else
        (Default|ExponentialJump _mover DeltaSeconds)))
    (else
      (Default|CoyoteGroundCheck _mover DeltaSeconds false))))