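; Mover component for side-on 2D character movement, driving a Collider in the X-Z plane from a 2D velocity.
; Tick resets jumps when grounded, applies gravity in the air, then moves each axis separately.
; Helpers provide acceleration and deceleration, multi-jump, box-trace ground and head checks, and coyote time.
; Physics, simple and exponential jump models have construct functions deriving jump velocity and gravity from jump height and time.
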(event EventTick
  (params (DeltaSeconds :type Float%20%28single-precision%29))
  (if (Variables|Default|GetOnGround)
    (Variables|Default|SetJumpCount (Variables|Default|GetMaxJumpCount))
    (Variables|Default|SetCan%20Jump true)
    (if (Variables|Default|GetJumpButton)
      (CallFunction|JumpStart))
    (bind _xdirection (CallFunction|GetYDirection))
    (if (< _xdirection 0.0)
      (CallFunction|ClearY))
    (elif (and (Variables|Default|GetIsGravityActive) (not (Variables|Default|GetIsJumping)))
      (CallFunction|ApplyGravity DeltaSeconds)))
  (CallFunction|ApplyMotion DeltaSeconds))

(fn ApplyMotion
  (params (DeltaSeconds :type Float%20%28single-precision%29))
  (bind _velocity (Variables|Default|GetVelocity))
  (bind _sweep (Variables|Default|GetSweep))
  (bind _collider (Variables|Default|GetCollider))
  (bind _returnvalue (* _velocity DeltaSeconds))
  (bind (_x _y) (Math|Vector2D|BreakVector2D _returnvalue))
  (Transformation|AddWorldOffset _collider (Math|Vector|MakeVector _x 0.0 0.0) _sweep false)
  (Transformation|AddWorldOffset _collider (Math|Vector|MakeVector 0.0 0.0 _y) _sweep false))

(fn ClearY
  (Variables|Default|SetVelocity (* (Variables|Default|GetVelocity) "(X=1.000000,Y=0.000000)")))

(fn ClearX
  (Variables|Default|SetVelocity (* (Variables|Default|GetVelocity) "(X=0.000000,Y=1.000000)")))

(fn SetX
  (params (X :type Float%20%28single-precision%29))
  (Variables|Default|SetVelocity (Math|Vector2D|MakeVector2D X (.Y (Math|Vector2D|BreakVector2D (Variables|Default|GetVelocity))))))

(fn SetY
  (params (Y :type Float%20%28single-precision%29))
  (Variables|Default|SetVelocity (Math|Vector2D|MakeVector2D (.X (Math|Vector2D|BreakVector2D (Variables|Default|GetVelocity))) Y)))

(fn XMotion
  (params (DeltaSeconds :type Float%20%28single-precision%29) (Input :type Float%20%28single-precision%29) (Dead%20Zone :type Float%20%28single-precision%29))
  (bind _xacceleration (Variables|Default|GetXAcceleration))
  (bind _returnvalue (* DeltaSeconds Input _xacceleration))
  (bind _xdirection (CallFunction|GetXDirection))
  (if (> (Math|Float|Absolute(Float) Input) Dead%20Zone)
    (bind _sign (CallFunction|GetSignValue _returnvalue))
    (CallFunction|ApproachV2X (Variables|Default|GetVelocity) _returnvalue (* (Variables|Default|GetMaxSpeedX) _sign))
    (else
      (CallFunction|GetSignValue (* (Variables|Default|GetXDeceleration) _xdirection -1.0 DeltaSeconds))
      (CallFunction|ApproachV2X (Variables|Default|GetVelocity) (* (Variables|Default|GetXDeceleration) _xdirection -1.0 DeltaSeconds) 0.0))))

(fn GetXDirection
  (bind _sign (CallFunction|GetSignValue (.X (Math|Vector2D|BreakVector2D (Variables|Default|GetVelocity)))))
  (return _sign))

(fn YMotion
  (params (DeltaSeconds :type Float%20%28single-precision%29) (Input :type Float%20%28single-precision%29) (Acceleration :type Float%20%28single-precision%29) (Deceleration :type Float%20%28single-precision%29) (Max%20Speed :type Float%20%28single-precision%29) (Dead%20Zone :type Float%20%28single-precision%29))
  (bind _returnvalue (* DeltaSeconds Input Acceleration))
  (bind _xdirection (CallFunction|GetYDirection))
  (if (> (Math|Float|Absolute(Float) Input) Dead%20Zone)
    (bind _sign (CallFunction|GetSignValue _returnvalue))
    (CallFunction|ApproachV2Y (Variables|Default|GetVelocity) _returnvalue (* Max%20Speed _sign))
    (else
      (bind _sign_2 (CallFunction|GetSignValue (* Deceleration _xdirection -1.0)))
      (CallFunction|ApproachV2Y (Variables|Default|GetVelocity) (* Deceleration _xdirection -1.0) (* Max%20Speed _sign_2)))))

(fn GetYDirection
  (bind _sign (CallFunction|GetSignValue (.Y (Math|Vector2D|BreakVector2D (Variables|Default|GetVelocity)))))
  (return _sign))

(fn GroundCheck
  (params (IgnorePermeable :type Boolean))
  (bind _collider (Variables|Default|GetCollider))
  (bind _returnvalue (Transformation|GetWorldLocation _collider))
  (bind _boxextent (Variables|/Script/Engine.BoxComponent|GetBoxExtent _collider))
  (bind _returnvalue_2 (* _boxextent "0.900000,0.900000, 0"))
  (bind _returnvalue_3 (* _boxextent "0, 0,1.000000"))
  (bind _returnvalue_4 (- _returnvalue _returnvalue_3))
  (bind _returnvalue_5 (- _returnvalue_4 "0, 0,2.000000"))
  (if IgnorePermeable
    (bind _returnvalue_6 (Class|KismetSystemLibrary|BoxTraceSingleforObjects _returnvalue_4 _returnvalue_5 _returnvalue_2 "0, 0, 0" (Utilities|Array|MakeArray "ObjectTypeQuery7") false 0 (Variables|Default|GetDebugTrace) true))
    (return _returnvalue_6)
    (else
      (bind _returnvalue_7 (Class|KismetSystemLibrary|BoxTraceSingleforObjects _returnvalue_4 _returnvalue_5 _returnvalue_2 "0, 0, 0" (Utilities|Array|MakeArray "ObjectTypeQuery7" "ObjectTypeQuery8") false 0 (Variables|Default|GetDebugTrace) true))
      (return _returnvalue_7))))

(fn CoyoteGroundCheck
  (params (DeltaSeconds :type Float%20%28single-precision%29) (IgnorePermeable :type Boolean))
  (bind _onground (CallFunction|GroundCheck IgnorePermeable))
  (if (not (Math|Boolean|Equal(Boolean) _onground (Variables|Default|GetOnGround)))
    (if (Math|Boolean|Equal(Boolean) _onground false)
      (if (> (Variables|Default|GetCoyoteTime) 0.0)
        (bind _output_get (Variables|Default|SetCoyoteTime (- (Variables|Default|GetCoyoteTime) DeltaSeconds)))
        (if (<= _output_get 0.0)
          (Variables|Default|SetOnGround false)
          (Variables|Default|SetCoyoteTime 0.0))
        (else
          (Variables|Default|SetCoyoteTime (Variables|Default|GetMaxCoyoteTime))))
      (else
        (Variables|Default|SetOnGround true)))))

(fn JumpStart
  (Variables|Default|SetJumpButton true)
  (if (Variables|Default|GetCan%20Jump)
    (Variables|Default|SetIsJumping true)
    (Variables|Default|SetStartJumpHeight (.Z (Math|Vector|BreakVector (Transformation|GetWorldLocation (Variables|Default|GetCollider)))))
    (Variables|Default|SetOnGround false)
    (bind _result (Math|Integer|DecrementInt (Variables|Default|GetJumpCount))
      (:%20%20
        (if (== _result 0)
          (Variables|Default|SetCan%20Jump false))))))

(fn JumpStop
  (Variables|Default|SetIsJumping false)
  (Variables|Default|SetJumpButton false))

(fn ApplyGravity
  (params (DeltaSeconds :type Float%20%28single-precision%29))
  (CallFunction|ApproachV2Y (Variables|Default|GetVelocity) (* DeltaSeconds (Variables|Default|GetGravity) -1.0) (* -1 (Variables|Default|GetTerminalVelocity))))

(fn PhysicsConstruct
  (params (TerminalVelocityMult :type Float%20%28single-precision%29))
  (bind _maxjumptime (Variables|Default|GetMaxJumpTime))
  (bind _output_get (Variables|Default|SetJumpVelocity (/ (* (Variables|Default|GetMaxJumpHeight) 4.0) _maxjumptime)))
  (bind _output_get_2 (Variables|Default|SetGravity (/ _output_get _maxjumptime)))
  (Variables|Default|SetTerminalVelocity (* _output_get_2 TerminalVelocityMult)))

(fn PhysicsJump
  (CallFunction|SetY (Variables|Default|GetJumpVelocity))
  (Variables|Default|SetIsJumping false))

(fn SimpleConstruct
  (params (TerminalVelocityMult :type Float%20%28single-precision%29) (JumpControlPercent :type Float%20%28single-precision%29))
  (bind _maxjumptime (Variables|Default|GetMaxJumpTime))
  (bind _maxjumptime_2 (Variables|Default|GetMaxJumpTime))
  (bind _output_get (Variables|Default|SetTrueMaxJump (* JumpControlPercent (Variables|Default|GetMaxJumpHeight))))
  (bind _output_get_2 (LocalVariables|SetTempHeightTime (/ (- _maxjumptime_2 (Math|Float|Sqrt (* (- JumpControlPercent 1.0) _maxjumptime_2 -1.0))) 2.0)))
  (bind _output_get_3 (Variables|Default|SetJumpVelocity (/ _output_get _output_get_2)))
  (bind _output_get_4 (Variables|Default|SetGravity (/ (+ _output_get_3 _output_get) (- _maxjumptime _output_get_2))))
  (Variables|Default|SetTerminalVelocity (* _maxjumptime TerminalVelocityMult _output_get_4)))

(fn SimpleJump
  (if (> (.Z (Math|Vector|BreakVector (Transformation|GetWorldLocation (Variables|Default|GetCollider)))) (+ (Variables|Default|GetStartJumpHeight) (Variables|Default|GetTrueMaxJump)))
    (Variables|Default|SetIsJumping false)
    (Variables|Default|SetOnGround false)
    (else
      (CallFunction|SetY (Variables|Default|GetJumpVelocity)))))

(fn ExponentialConstruct
  (params (TerminalVelocityMult :type Float%20%28single-precision%29) (JumpControlPercent :type Float%20%28single-precision%29))
  (bind _maxjumptime (Variables|Default|GetMaxJumpTime))
  (bind _maxjumptime_2 (Variables|Default|GetMaxJumpTime))
  (bind _output_get (Variables|Default|SetTrueMaxJump (* JumpControlPercent (Variables|Default|GetMaxJumpHeight))))
  (bind _output_get_2 (LocalVariables|SetTempHeightTime (/ (- _maxjumptime_2 (Math|Float|Sqrt (* (- JumpControlPercent 1.0) _maxjumptime_2 -1.0))) 2.0)))
  (bind _output_get_3 (Variables|Default|SetJumpVelocity (/ _output_get (Math|Float|Power _output_get_2 3.0))))
  (bind _output_get_4 (Variables|Default|SetGravity (/ (+ _output_get_3 _output_get) (- _maxjumptime _output_get_2))))
  (Variables|Default|SetTerminalVelocity (* _maxjumptime TerminalVelocityMult _output_get_4)))

(fn ExponentialJump
  (params (DeltaSeconds :type Float%20%28single-precision%29))
  (if (> (.Z (Math|Vector|BreakVector (Transformation|GetWorldLocation (Variables|Default|GetCollider)))) (+ (Variables|Default|GetStartJumpHeight) (Variables|Default|GetTrueMaxJump)))
    (Variables|Default|SetIsJumping false)
    (Variables|Default|SetOnGround false)
    (else
      (CallFunction|SetY (+ (* DeltaSeconds (Variables|Default|GetJumpVelocity)) (.Y (Math|Vector2D|BreakVector2D (Variables|Default|GetVelocity))))))))

(fn XConstruct
  (bind _maxspeedx (Variables|Default|GetMaxSpeedX))
  (Variables|Default|SetXAcceleration (/ _maxspeedx (Variables|Default|GetTimeToStartX)))
  (Variables|Default|SetXDeceleration (/ _maxspeedx (Variables|Default|GetTimeToStopX))))

(fn HeadCheck
  (bind _collider (Variables|Default|GetCollider))
  (bind _returnvalue (Transformation|GetWorldLocation _collider))
  (bind _boxextent (Variables|/Script/Engine.BoxComponent|GetBoxExtent _collider))
  (bind _returnvalue_2 (* _boxextent "0, 0,1.000000"))
  (bind _returnvalue_3 (+ _returnvalue _returnvalue_2))
  (bind _returnvalue_4 (Class|KismetSystemLibrary|BoxTraceSingleforObjects _returnvalue_3 (+ _returnvalue_3 "0, 0,2.000000") (* _boxextent "0.900000,0.900000, 0") "0, 0, 0" (Utilities|Array|MakeArray "ObjectTypeQuery7") false 0 (Variables|Default|GetDebugTrace) true))
  (if _returnvalue_4
    (Variables|Default|SetIsJumping false)))

(fn GetJumpCount
  (return (Variables|Default|GetMaxJumpCount)))

(fn SetJumpCount
  (params (JumpCount :type Integer))
  (Variables|Default|SetMaxJumpCount JumpCount))