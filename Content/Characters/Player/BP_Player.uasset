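; Player character Blueprint for a platformer that routes player input to movement, jump and interaction components.
; The construction script gives the mover its ground collider, links it to the platformer controller and caches the sprite's initial X scale.
; Horizontal input feeds the controller and flips the sprite via the sign of its X scale.
; An IgnoreInput flag zeroes movement and blocks jump starts, while Quit exits the game.
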(event Input|ActionEvents|InputActionJump
  (params (Key :type Key%20Structure :default "None"))
  (bind _bp_ac_mover (Variables|Default|GetBP_AC_Mover))
  (:Pressed
    (if (not (Variables|Default|GetIgnoreInput))
      (Default|JumpStart _bp_ac_mover)))
  (:Released
    (Default|JumpStop _bp_ac_mover)))

(event Input|ActionEvents|InputActionInteract
  (params (Key :type Key%20Structure :default "None"))
  (:Pressed
    (Default|Interact (Variables|Default|GetBP_AC_Interactor))))

(event Input|ActionEvents|InputActionQuit
  (params (Key :type Key%20Structure :default "None"))
  (:Pressed
    (Game|QuitGame 0 "Quit" false)))

(event Input|AxisEvents|InputAxisMoveRight
  (params (AxisValue :type Float%20%28single-precision%29))
  (bind _bp_ac_platformercontroller (Variables|Default|GetBP_AC_PlatformerController))
  (bind _sprite (Variables|Default|GetSprite))
  (bind _returnvalue (Transformation|GetWorldScale _sprite))
  (bind (_x _y _z) (Math|Vector|BreakVector _returnvalue))
  (if (Variables|Default|GetIgnoreInput)
    (Variables|/Game/Characters/Blueprints/BP_AC_PlatformerController.BP_AC_PlatformerController_C|SetX%20Input _bp_ac_platformercontroller 0.0)
    (else
      (bind _output_get (Variables|/Game/Characters/Blueprints/BP_AC_PlatformerController.BP_AC_PlatformerController_C|SetX%20Input _bp_ac_platformercontroller AxisValue))
      (if (not (== _output_get 0.0))
        (bind _sign (CallFunction|GetSignValue _output_get))
        (Transformation|SetWorldScale3D _sprite (Math|Vector|MakeVector (* _sign (Variables|Default|GetInitialSpriteXScale)) _y _z))))))

(fn ConstructionScript
  (bind _bp_ac_mover (Variables|Default|GetBP_AC_Mover))
  (Variables|/Game/Characters/Blueprints/BP_AC_Mover.BP_AC_Mover_C|SetCollider _bp_ac_mover (Variables|Default|GetGround%20Collider))
  (Variables|/Game/Characters/Blueprints/BP_AC_PlatformerController.BP_AC_PlatformerController_C|SetMover (Variables|Default|GetBP_AC_PlatformerController) _bp_ac_mover)
  (Variables|Default|SetInitialSpriteXScale (.X (Math|Vector|BreakVector (Transformation|GetWorldScale (Variables|Default|GetSprite))))))